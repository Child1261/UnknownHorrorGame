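; BP_Entity is the player-controlled monster character that hunts BP_Expunger players in a multiplayer game.
; Interact runs a server-to-multicast attack that boosts speed and repeats a timed sphere trace until it damages an Expunger or times out, followed by a slowdown and cooldown.
; Abilities spawn an arrow toward the nearest living Expunger, web projectiles and web traps.
; Look-at rotation replicates via server and multicast events.
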(event Custom|Server_Attack
  (bind _self self)
  (bind _playercontroller (Variables|Default|GetPlayerController))
  (bind _attack_trace (Variables|Default|GetAttack%20Trace))
  (bind _returnvalue (Transformation|GetWorldLocation _attack_trace))
  (Default|ChangeEntitySpeed (Variables|Default|GetPlayerController) self (+ (Variables|Default|GetdefaultMoveSpeed) (Variables|Default|GetattackSpeedModifier)))
  (bind (_outhit _returnvalue_2) (Collision|SphereTraceForObjects _returnvalue (+ _returnvalue (* (Math|Vector|GetForwardVector (Transformation|GetWorldRotation _attack_trace)) 5e+01)) 5e+01 (Utilities|Array|MakeArray "ObjectTypeQuery3") false (Variables|Default|GetActors%20to%20Ignore) "None"))
  (if _returnvalue_2
    (Default|ChangeHitPlayer _playercontroller true _self)
    (CallFunction|ServerHarmPlayer (.hitactor _outhit))
    (Utilities|Array|Add (Variables|Default|GetActors%20to%20Ignore) (.hitactor _outhit))
    (Variables|Default|SetAttacking false)
    (Utilities|Time|ClearandInvalidateTimerbyHandle (stale Custom|mc_initattack _returnvalue))
    (else
      (Default|ChangeHitPlayer _playercontroller false _self)))
  (Variables|Default|SetonAttackCooldown true))

(event Custom|CreateHUD
  (bind _asbp_player_controller (Utilities|Casting|CastToBP_PlayerController (Pawn|GetController)))
  (Default|CreateEntityHUD _asbp_player_controller (Variables|Default|GetInventorySystem)))

(event Custom|LocateNearestPlayer
  (bind _asbp__gamemode (Utilities|Casting|CastToBP__Gamemode (Game|GetGameMode)))
  ;[1 1 1] Gross hack, make sure closest is not null
  (bind _outactors (Actor|GetAllActorsOfClass "/Game/Character/Characters/BP_Expunger.BP_Expunger_C"))
  (Variables|Default|SetcurrentClosestExpunger (Utilities|Array|Get(acopy) _outactors))
  (for _array_element (Variables|/Game/Framework/BP__Gamemode.BP__Gamemode_C|GetAll_Player_Controllers _asbp__gamemode)
    (if (!= _array_element self)
      (bind _asbp_expunger (Utilities|Casting|CastToBP_Expunger (Pawn|GetControlledPawn _array_element)))
      (if (Variables|/Game/Character/Characters/BP_Expunger.BP_Expunger_C|GetisAlive _asbp_expunger)
        (CallFunction|FindClosestPlayer _asbp_expunger))))
  (CallFunction|CreateArrow))

(event Custom|server_initattack
  (CallFunction|McInitattack))

(event Custom|mc_initattack
  (if (and (not (Variables|Default|GetAttacking)) (not (Variables|Default|GetonAttackCooldown)))
    (Utilities|Array|Clear (Variables|Default|GetActors%20to%20Ignore))
    (Variables|Default|SetAttacking true)
    (bind _returnvalue (Utilities|Time|SetTimerbyEvent (delegate Custom|Server_Attack) 0.1 true))
    (Utilities|FlowControl|Delay (Variables|Default|GetattackDuration))
    (Utilities|Time|ClearandInvalidateTimerbyHandle _returnvalue)
    (Variables|Default|SetAttacking false)
    (CallFunction|HandleCooldown)))

(event Custom|findClosestPlayer
  (params (Expunger :type BP%20Expunger%20Object%20Reference))
  (if (Utilities|IsValid (Variables|Default|GetcurrentClosestExpunger))
    (if (< (Transformation|GetDistanceTo Expunger self) (Transformation|GetDistanceTo (Variables|Default|GetcurrentClosestExpunger) self))
      (Variables|Default|SetcurrentClosestExpunger Expunger))))

(event Custom|createArrow
  (Game|SpawnActorfromClass "/Game/Character/Characters/Inventory/items/SpiderPowers/Locate/PointAtPlayer.PointAtPlayer_C" (Transformation|GetWorldTransform (Variables|Default|GetAttack%20Trace)) "Undefined" "MultiplyWithRoot" 0 (Variables|Default|GetcurrentClosestExpunger) self 0))

(event Custom|setLightVisible
  (Rendering|SetVisibility (Variables|Default|GetSpotLight) true false))

(event Custom|Server_Rotation
  (params (New%20Direction :type Rotator))
  (CallFunction|RotationMultiCast New%20Direction))

(event Custom|Rotation_MultiCast
  (params (newDirection :type Rotator))
  (bind _returnvalue (Pawn|GetController))
  (Utilities|IsValid _returnvalue
    (:Is%20Valid
      (Pawn|SetControlRotation _returnvalue newDirection))))

(event Custom|handleCooldown
  (bind _playercontroller (Variables|Default|GetPlayerController))
  (if (Variables|Default|GethitPlayer?)
    (Default|ChangeEntitySpeed _playercontroller self (- (Variables|Default|GetdefaultMoveSpeed) (Variables|Default|GethitSlowdownSpeed)))
    (Utilities|FlowControl|Delay (Variables|Default|GetmissPenaltyDuration))
    (else
      (Default|ChangeEntitySpeed _playercontroller self (- (Variables|Default|GetdefaultMoveSpeed) (Variables|Default|GetmissPenaltyModifer)))
      (Utilities|FlowControl|Delay (Variables|Default|GetmissPenaltyDuration))))
  (Default|ChangeEntitySpeed (Variables|Default|GetPlayerController) self (Variables|Default|GetdefaultMoveSpeed))
  (Utilities|FlowControl|Delay (Variables|Default|GetattackCooldown))
  (Variables|Default|SetonAttackCooldown false))

(event Custom|Server_harmPlayer
  (params (Out%20Hit%20Hit%20Actor :type Actor%20Object%20Reference))
  (bind _asbp_expunger (Utilities|Casting|CastToBP_Expunger Out%20Hit%20Hit%20Actor))
  (Default|DamagePlayer _asbp_expunger (Variables|Default|GetattackDamage)))

(event Custom|FireWeb
  (Game|SpawnActorfromClass "/Game/Character/Characters/Inventory/items/SpiderPowers/WebShoot/WebProjectile.WebProjectile_C" (Transformation|GetWorldTransform (Variables|Default|GetAttack%20Trace)) "AlwaysSpawn" "MultiplyWithRoot" 0 0))

(event Custom|LayWebTrap
  (Game|SpawnActorfromClass "/Game/Character/Characters/Inventory/items/SpiderPowers/WebTrap/WebTrapPlaceable.WebTrapPlaceable_C" (Math|Transform|MakeTransform (- (Transformation|GetActorLocation) "0.000000,0.000000,40.000000") (Math|Rotator|MakeRotator 0.0 0.0 (+ (.yaw (Math|Rotator|MakeRotfromX (Transformation|GetActorForwardVector))) 9e+01 0.0)) "1.000000,1.000000,1.000000") "AlwaysSpawn" "MultiplyWithRoot" 0 0))

(event Custom|Server_putOnCooldown
  (CallFunction|MCPutonCooldown))

(event Custom|MC_putOnCooldown
  (Variables|Default|SetonAbilityCooldown? true)
  (Utilities|FlowControl|Delay 5.0)
  (Variables|Default|SetonAbilityCooldown? false))

(event Input|EnhancedActionEvents|EnhancedInputActionIA_Interact
  (params (ActionValue :type Boolean) (ElapsedSeconds :type Float%20%28double-precision%29) (TriggeredSeconds :type Float%20%28double-precision%29) (InputAction :type Input%20Action%20Object%20Reference :default "/Game/Character/Characters/Inputs/Actions/IA_Interact.IA_Interact"))
  (:Started
    (bind _asbp_player_controller (Utilities|Casting|CastToBP_PlayerController (Pawn|GetController)))
    (Default|SetController _asbp_player_controller self)
    (CallFunction|ServerInitattack)))

(event EventBeginPlay
  (bind _asplayer_controller (Utilities|Casting|CastToPlayerController (Pawn|GetController)))
  (Utilities|IsValid (PlayerController|LocalPlayerSubsystems|GetEnhancedInputLocalPlayerSubsystem _asplayer_controller)
    (:Is%20Valid
      (Input|AddMappingContext (PlayerController|LocalPlayerSubsystems|GetEnhancedInputLocalPlayerSubsystem _asplayer_controller) "/Game/Character/Characters/Inputs/InputMapping.InputMapping" 0 "(bIgnoreAllPressedKeysUntilRelease=True,bForceImmediately=False,bNotifyUserSettings=False)")
      (CallFunction|SetLightVisible))))

(event EventLookat
  (params (direction :type Vector :default "0, 0, 0") (Actor :type Actor%20Object%20Reference))
  (bind _returnvalue (Transformation|GetActorLocation))
  (bind _returnvalue_2 (Transformation|GetActorLocation))
  (Networking|SwitchHasAuthority
    (:Authority
      _)
    (:Remote
      (CallFunction|ServerRotation (Math|Rotator|FindLookatRotation (Math|Vector|MakeVector (.x _returnvalue) (.y _returnvalue) 0.0) (Math|Vector|MakeVector (.x direction) (.y direction) 0.0)))))
  (CallFunction|RotationMultiCast (Math|Rotator|FindLookatRotation (Math|Vector|MakeVector (.x _returnvalue_2) (.y _returnvalue_2) 0.0) (Math|Vector|MakeVector (.x direction) (.y direction) 0.0))))

(fn ConstructionScript
  (bind _los_comp (Variables|Default|GetLos_Comp))
  (Variables|/Game/LineOfSightMP/BP/AC_Los.AC_Los_C|SetPointLight _los_comp 0)
  (Variables|/Game/LineOfSightMP/BP/AC_Los.AC_Los_C|SetSpotLight _los_comp 0))