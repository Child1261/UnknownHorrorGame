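; Player controller for a cursor-aimed pawn that also handles lobby UI and leaving a session.
; Enhanced Input drives movement along world axes, with the mouse cursor shown.
; Every tick it sends the pawn a look-at message through a collapsed graph, apparently for cursor-based facing.
; CreateLobby caches and displays the Pregame widget, while EndClientSession destroys the session and returns to MainMenu; the CreateLobbyWidget event is empty.
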(event Custom|CreateLobbyWidget)

(event Custom|EndClientSession
  (|DestroySession self
    (:then
      (Game|OpenLevel(byName) "MainMenu"))))

(event Input|EnhancedActionEvents|EnhancedInputActionIA_Move
  (params (ActionValue :type Vector%202D%20Structure) (ElapsedSeconds :type Float%20%28double-precision%29) (TriggeredSeconds :type Float%20%28double-precision%29) (InputAction :type Input%20Action%20Object%20Reference :default "/Game/Character/Characters/Inputs/Actions/IA_Move.IA_Move"))
  ;[1 1 1] Movement
  (:Triggered
    (Pawn|Input|AddMovementInput (Pawn|GetControlledPawn) (Math|Vector|GetRightVector (Math|Rotator|MakeRotator 0.0 0.0 0.0)) (.x ActionValue) false)
    (Pawn|Input|AddMovementInput (Pawn|GetControlledPawn) (Math|Vector|GetForwardVector (Math|Rotator|MakeRotator 0.0 0.0 0.0)) (.y ActionValue) false)))

(event EventTick
  (params (DeltaSeconds :type Float%20%28single-precision%29))
  (CallFunction|HandlePlayerRotation))

(event EventBeginPlay
  (bind _returnvalue (PlayerController|LocalPlayerSubsystems|GetEnhancedInputLocalPlayerSubsystem))
  (Utilities|IsValid _returnvalue
    (:Is%20Valid
      (Input|AddMappingContext _returnvalue 0 0 "(bIgnoreAllPressedKeysUntilRelease=True,bForceImmediately=False)")
      (Variables|Default|SetbShowMouseCursor true))))

(fn ConstructionScript)

(fn GetLocationUnderCursor
  (return (.Location (Collision|BreakHitResult (.HitResult (Game|Player|GetHitResultUnderCursorbyChannel "TraceTypeQuery1" true))))))

(fn HandlePlayerRotation
  (Class|BPIPlayer|Lookat(Message) (Pawn|GetControlledPawn) (|CollapseGraph)))

(fn CreateLobby
  (Utilities|IsValid (Variables|Default|GetWB_LobbyMenu)
    (:Is%20Valid
      _)
    (:Is%20Not%20Valid
      (bind _returnvalue (UserInterface|CreateWidget "/Game/UI/InGame/Pre-game/Pregame.Pregame_C" self))
      (Variables|Default|SetWB_LobbyMenu _returnvalue)))
  (UserInterface|Viewport|AddtoViewport (Variables|Default|GetWB_LobbyMenu) 0)
  (return))