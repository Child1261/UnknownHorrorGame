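; Game mode for an asymmetric multiplayer lobby and match, with one player as the Entity and the rest as Expungers.
; Login and logout maintain the controller list, which a looping timer and delayed update push to BP_GameState to build the lobby.
; StartGame leaves the lobby, clears existing Expungers, spawns and possesses pawns by the selected index, and resets UI and input.
; Helpers kick players or swap one into a new Entity pawn.
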(event Custom|UpdateLobby
  (if (Variables|Default|GetInLobby)
    ;[1 1 1] Ensure one player is entity
    (if (>= (Variables|Default|GetSelectedPlayer) (Utilities|Array|Length (Variables|Default|GetAll_Player_Controllers)))
      (Variables|Default|SetSelectedPlayer 0))
    (CallFunction|UpdateList)
    (else
      (Utilities|Time|ClearandInvalidateTimerbyHandle (stale EventBeginPlay _returnvalue)))))

(event Custom|Update_List
  (Utilities|FlowControl|Delay 0.3)
  (bind _asbp_game_state (Utilities|Casting|CastToBP_GameState (Game|GetGameState)))
  (Default|GenerateLobby _asbp_game_state (Variables|Default|GetAll_Player_Controllers) (Variables|Default|GetSelectedPlayer)))

(event EventBeginPlay
  (bind _returnvalue (Utilities|Time|SetTimerbyEvent (delegate Custom|UpdateLobby) 0.5 true)))

(event EventPostLogin
  (params (NewPlayer :type Player%20Controller%20Object%20Reference))
  (bind _asbp_player_controller (Utilities|Casting|CastToBP_PlayerController NewPlayer))
  (Utilities|Array|Add (Variables|Default|GetAll_Player_Controllers) _asbp_player_controller)
  (CallFunction|UpdateList))

(event EventOnLogout
  (params (ExitingController :type Controller%20Object%20Reference))
  (bind _asbp_player_controller (Utilities|Casting|CastToBP_PlayerController ExitingController))
  (Utilities|Array|RemoveItem (Variables|Default|GetAll_Player_Controllers) _asbp_player_controller)
  (CallFunction|UpdateList))

(fn ConstructionScript)

(fn KickPlayer
  (params (Player%20ID :type Integer))
  (Class|AdvancedSessionsLibrary|KickPlayer (Game|GetPlayerController Player%20ID) "Get kicked scrub")
  (Variables|Default|SetSelectedPlayer 0))

(fn UpdatePlayerList)

(fn SetEntity
  (params (PlayerID :type Integer))
  (bind _returnvalue (Game|GetPlayerController PlayerID))
  (bind _returnvalue_2 (Pawn|GetControlledPawn _returnvalue))
  (Utilities|IsValid _returnvalue
    (:Is%20Valid
      (Utilities|IsValid _returnvalue_2
        (:Is%20Valid
          (Actor|DestroyActor _returnvalue_2)
          (bind _returnvalue_3 (Game|SpawnActorfromClass "/Game/Character/Characters/BP_Entity.BP_Entity_C" (Math|Transform|MakeTransform "0, 0, 0" "0, 0, 0" "1.000000,1.000000,1.000000") "Undefined" "MultiplyWithRoot" 0 0))
          (Pawn|Possess _returnvalue _returnvalue_3))))))

(fn StartGame
  ;[1 1 1] Make sure no exisiting actors
  (Variables|Default|SetInLobby false)
  (bind _outactors (Actor|GetAllActorsOfClass "/Game/Character/Characters/BP_Expunger.BP_Expunger_C"))
  (for _array_element _outactors
    (Actor|DestroyActor _array_element))
  (for (_array_element_2 _array_index) (Variables|Default|GetAll_Player_Controllers)
    (if (== _array_index (Variables|Default|GetSelectedPlayer))
      (bind _returnvalue (Game|SpawnActorfromClass "/Game/Character/Characters/BP_Entity.BP_Entity_C" (Math|Transform|MakeTransform "0, 0, 0" "0, 0, 0" "1.000000,1.000000,1.000000") "AdjustIfPossibleButDontSpawnIfColliding" "MultiplyWithRoot" 0 0))
      (Pawn|Possess _array_element_2 _returnvalue)
      (else
        (bind _returnvalue_2 (Game|SpawnActorfromClass "/Game/Character/Characters/BP_Expunger.BP_Expunger_C" (Math|Transform|MakeTransform "0, 0, 0" "0, 0, 0" "1.000000,1.000000,1.000000") "Undefined" "MultiplyWithRoot" 0 0))
        (Pawn|Possess _array_element_2 _returnvalue_2)))
    (Viewport|RemoveAllWidgets)
    (Utilities|Casting|CastToBP_GameState (Game|GetGameState))
    (for _array_element_3 (Variables|Default|GetAll_Player_Controllers)
      (Input|SetInputModeGameandUI _array_element_3 0 "DoNotLock" false false))))