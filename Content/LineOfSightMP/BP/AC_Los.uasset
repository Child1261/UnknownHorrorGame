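; Line-of-sight component that draws what its pawn can see into a per-player render target, for top-down or side views in multiplayer.
; Setup picks target and body color by PlayerID, configures lights and MPC_Los, and disables LOS on pawn materials.
; Each locally controlled tick line-traces a fan, then draws the hits as canvas triangles.
; Traces ignore "LOS"-tagged actors; "Loshit" tags extend vision past hits.
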(event Custom|Update
  (params (PlayerID :type Integer))
  (bind _returnvalue (Components|GetOwner))
  (bind _spotlight (Variables|IgnoreMe|GetSpotLight))
  (bind _aspawn (Utilities|Casting|CastToPawn _returnvalue))
  (Variables|IgnoreMe|SetPlayerID PlayerID)
  (Utilities|FlowControl|Sequence
    (:then_0
      ;[1 1 1] If you have a single-user project, you can disable these parts.
      (if (>= (Variables|IgnoreMe|GetPlayerID) 0)
        (Variables|IgnoreMe|SetLosRenderTarget (Utilities|Select :Index (Variables|IgnoreMe|GetPlayerID) :Option%200 "/Game/LineOfSightMP/Textures/RTC_LOS0.RTC_LOS0" :Option%201 "/Game/LineOfSightMP/Textures/RTC_LOS1.RTC_LOS1" :Option%202 "/Game/LineOfSightMP/Textures/RTC_LOS2.RTC_LOS2" :Option%203 "/Game/LineOfSightMP/Textures/RTC_LOS3.RTC_LOS3" :Option%204 "/Game/LineOfSightMP/Textures/RTC_LOS4.RTC_LOS4" :Option%205 "/Game/LineOfSightMP/Textures/RTC_LOS5.RTC_LOS5" :Option%206 "/Game/LineOfSightMP/Textures/RTC_LOS6.RTC_LOS6" :Option%207 "/Game/LineOfSightMP/Textures/RTC_LOS7.RTC_LOS7"))
        (bind _ascharacter (Utilities|Casting|CastToCharacter (Components|GetOwner)))
        (Rendering|Material|SetVectorParameterValueonMaterials (Variables|/Script/Engine.Character|GetMesh _ascharacter) "BodyColor" (Utilities|Select :Index (Variables|IgnoreMe|GetPlayerID) :Option%200 "1.000000, 0, 0" :Option%201 "0,1.000000, 0" :Option%202 "0, 0,1.000000" :Option%203 "1.000000,1.000000, 0" :Option%204 "0,1.000000,1.000000" :Option%205 "1.000000,1.000000,1.000000" :Option%206 "1.000000, 0,1.000000" :Option%207 "0.500000,1.000000, 0"))))
    (:then_1
      (if (Variables|Default|GetFovMP)
        (Utilities|FlowControl|Sequence
          (:then_0
            (if (Pawn|IsLocallyControlled (.AsPawn (Utilities|Casting|CastToPawn (Components|GetOwner)))) :!label _label
              (Utilities|FlowControl|Sequence
                (:then_0
                  ;[1 1 1] These actors will be ignored in CreateVision
                  (bind _outactors (Actor|GetAllActorswithTag "LOS"))
                  (Variables|IgnoreMe|SetLOSActors _outactors)
                  (Utilities|FlowControl|Sequence
                    (:then_1
                      (if (Variables|Default|GetFovMP)
                        ;;[1 1 1] All Players
                        (bind _outactors_2 (Actor|GetAllActorsOfClass (Utilities|GetClass _aspawn)))
                        (for _array_element _outactors_2
                          (CallFunction|DisableforPlayer _array_element))
                        (else
                          (CallFunction|DisableforPlayer _aspawn) ; Self Only
                        )))))
                (:then_1
                  (if (not (Variables|Default|GetFovMP))
                    ;[1 1 1] Setting the light
                    (Utilities|IsValid (Variables|IgnoreMe|GetPointLight) :!label _label_2
                      (:Is%20Valid
                        (Utilities|IsValid (Variables|IgnoreMe|GetSpotLight)
                          (:Is%20Valid
                            (Rendering|Lighting|SetAttenuationRadius (Variables|IgnoreMe|GetPointLight) (+ (Variables|Default|GetDistance) 25.0))
                            (if (>= (Variables|Default|GetAngle) 150)
                              (Variables|Default|SetAngle 360)
                              (Rendering|SetVisibility (Variables|IgnoreMe|GetPointLight) true false)
                              (Rendering|SetVisibility (Variables|IgnoreMe|GetSpotLight) false false)
                              (else
                                (Rendering|SetVisibility (Variables|IgnoreMe|GetPointLight) false false)
                                (Rendering|SetVisibility _spotlight true false)
                                (Rendering|Lighting|SetOuterConeAngle _spotlight (+ (Math|Conversions|ToFloat(Integer) (/ (Variables|Default|GetAngle) 2)) 4.0))
                                (Rendering|Lighting|SetInnerConeAngle _spotlight 0.0)))))))))
                (:then_2
                  ;[1 1 1] Data transmission to materials
                  (Rendering|Material|SetScalarParameterValue "/Game/LineOfSightMP/Materials/MPC_Los.MPC_Los" "TopDown" (Utilities|Select :Index (Variables|Default|GetLosType) :NewEnumerator0 1.0 :NewEnumerator1 0.0) :!class /Script/Engine.KismetMaterialLibrary)
                  (Rendering|Material|SetScalarParameterValue "/Game/LineOfSightMP/Materials/MPC_Los.MPC_Los" "GlobalEnable" 1.0 :!class /Script/Engine.KismetMaterialLibrary)
                  (Rendering|Material|SetScalarParameterValue "/Game/LineOfSightMP/Materials/MPC_Los.MPC_Los" "PlayerID" (Math|Conversions|ToFloat(Integer) (Variables|IgnoreMe|GetPlayerID)) :!class /Script/Engine.KismetMaterialLibrary)
                  (Rendering|Material|SetScalarParameterValue "/Game/LineOfSightMP/Materials/MPC_Los.MPC_Los" "Distance" (Variables|Default|GetDistance) :!class /Script/Engine.KismetMaterialLibrary)))))
          (:then_1
            (goto _label_2)))
        (else
          (goto _label))))))

(event EventBeginPlay
  (bind _returnvalue (Components|GetOwner))
  (bind _playerid (Variables|IgnoreMe|GetPlayerID))
  (bind _spotlight (Variables|IgnoreMe|GetSpotLight))
  (bind _aspawn (Utilities|Casting|CastToPawn _returnvalue))
  (Utilities|FlowControl|Sequence
    (:then_0
      ;[1 1 1] If you have a single-user project, you can disable these parts.
      (if (>= _playerid 0)
        (Variables|IgnoreMe|SetLosRenderTarget (Utilities|Select :Index _playerid :Option%200 "/Game/LineOfSightMP/Textures/RTC_LOS0.RTC_LOS0" :Option%201 "/Game/LineOfSightMP/Textures/RTC_LOS1.RTC_LOS1" :Option%202 "/Game/LineOfSightMP/Textures/RTC_LOS2.RTC_LOS2" :Option%203 "/Game/LineOfSightMP/Textures/RTC_LOS3.RTC_LOS3" :Option%204 "/Game/LineOfSightMP/Textures/RTC_LOS4.RTC_LOS4" :Option%205 "/Game/LineOfSightMP/Textures/RTC_LOS5.RTC_LOS5" :Option%206 "/Game/LineOfSightMP/Textures/RTC_LOS6.RTC_LOS6" :Option%207 "/Game/LineOfSightMP/Textures/RTC_LOS7.RTC_LOS7"))
        (bind _ascharacter (Utilities|Casting|CastToCharacter (Components|GetOwner)))
        (Rendering|Material|SetVectorParameterValueonMaterials (Variables|/Script/Engine.Character|GetMesh _ascharacter) "BodyColor" (Utilities|Select :Index _playerid :Option%200 "1.000000, 0, 0" :Option%201 "0,1.000000, 0" :Option%202 "0, 0,1.000000" :Option%203 "1.000000,1.000000, 0" :Option%204 "0,1.000000,1.000000" :Option%205 "1.000000,1.000000,1.000000" :Option%206 "1.000000, 0,1.000000" :Option%207 "0.500000,1.000000, 0"))))
    (:then_1
      (if (Variables|Default|GetFovMP)
        (Utilities|FlowControl|Sequence
          (:then_0
            (if (Pawn|IsLocallyControlled (.AsPawn (Utilities|Casting|CastToPawn (Components|GetOwner)))) :!label _label
              (Utilities|FlowControl|Sequence
                (:then_0
                  ;[1 1 1] These actors will be ignored in CreateVision
                  (bind _outactors (Actor|GetAllActorswithTag "LOS"))
                  (Variables|IgnoreMe|SetLOSActors _outactors)
                  (Utilities|FlowControl|Sequence
                    (:then_1
                      (if (Variables|Default|GetFovMP)
                        ;;[1 1 1] All Players
                        (bind _outactors_2 (Actor|GetAllActorsOfClass (Utilities|GetClass _aspawn)))
                        (for _array_element _outactors_2
                          (CallFunction|DisableforPlayer _array_element))
                        (else
                          (CallFunction|DisableforPlayer _aspawn) ; Self Only
                        )))))
                (:then_1
                  (if (not (Variables|Default|GetFovMP))
                    ;[1 1 1] Setting the light
                    (Utilities|IsValid (Variables|IgnoreMe|GetPointLight) :!label _label_2
                      (:Is%20Valid
                        (Utilities|IsValid (Variables|IgnoreMe|GetSpotLight)
                          (:Is%20Valid
                            (Rendering|Lighting|SetAttenuationRadius (Variables|IgnoreMe|GetPointLight) (+ (Variables|Default|GetDistance) 25.0))
                            (if (>= (Variables|Default|GetAngle) 150)
                              (Variables|Default|SetAngle 360)
                              (Rendering|SetVisibility (Variables|IgnoreMe|GetPointLight) true false)
                              (Rendering|SetVisibility (Variables|IgnoreMe|GetSpotLight) false false)
                              (else
                                (Rendering|SetVisibility (Variables|IgnoreMe|GetPointLight) false false)
                                (Rendering|SetVisibility _spotlight true false)
                                (Rendering|Lighting|SetOuterConeAngle _spotlight (+ (Math|Conversions|ToFloat(Integer) (/ (Variables|Default|GetAngle) 2)) 4.0))
                                (Rendering|Lighting|SetInnerConeAngle _spotlight 0.0)))))))))
                (:then_2
                  ;[1 1 1] Data transmission to materials
                  (Rendering|Material|SetScalarParameterValue "/Game/LineOfSightMP/Materials/MPC_Los.MPC_Los" "TopDown" (Utilities|Select :Index (Variables|Default|GetLosType) :NewEnumerator0 1.0 :NewEnumerator1 0.0) :!class /Script/Engine.KismetMaterialLibrary)
                  (Rendering|Material|SetScalarParameterValue "/Game/LineOfSightMP/Materials/MPC_Los.MPC_Los" "GlobalEnable" 1.0 :!class /Script/Engine.KismetMaterialLibrary)
                  (Rendering|Material|SetScalarParameterValue "/Game/LineOfSightMP/Materials/MPC_Los.MPC_Los" "PlayerID" (Math|Conversions|ToFloat(Integer) (Variables|IgnoreMe|GetPlayerID)) :!class /Script/Engine.KismetMaterialLibrary)
                  (Rendering|Material|SetScalarParameterValue "/Game/LineOfSightMP/Materials/MPC_Los.MPC_Los" "Distance" (Variables|Default|GetDistance) :!class /Script/Engine.KismetMaterialLibrary)))))
          (:then_1
            (goto _label_2)))
        (else
          (goto _label))))))

(event EventTick
  (params (DeltaSeconds :type Float%20%28single-precision%29))
  ;[1 1 1] LOS, EventTick
  (Variables|IgnoreMe|GetLosRenderTarget
    (:then
      (if (Pawn|IsLocallyControlled (.AsPawn (Utilities|Casting|CastToPawn (Components|GetOwner))))
        (Utilities|FlowControl|Sequence
          (:then_0
            (Rendering|Material|SetVectorParameterValue "/Game/LineOfSightMP/Materials/MPC_Los.MPC_Los" "PlayerPos" (Math|Conversions|ToLinearColor(Vector) (Transformation|GetActorLocation (Components|GetOwner))) :!class /Script/Engine.KismetMaterialLibrary))
          (:then_1
            (CallFunction|CreateVision)))))
    (:else)))

(fn CreateVision
  (bind _returnvalue (Components|GetOwner))
  (bind _returnvalue_2 (Components|GetOwner))
  (bind _returnvalue_3 (Components|GetOwner))
  (bind _returnvalue_4 (Math|Vector|MakeVector 9e+02 9e+02 9e+02))
  (bind _losrendertarget (Variables|IgnoreMe|GetLosRenderTarget))
  (bind _lostype (Variables|Default|GetLosType))
  (bind _distance (Variables|Default|GetDistance))
  (bind _angle (Variables|Default|GetAngle))
  (bind _angle_2 (Variables|Default|GetAngle))
  (bind _pitch (Variables|IgnoreMe|GetPitch))
  (bind _lostype_2 (Variables|Default|GetLosType))
  (bind _traceresult (LocalVariables|GetTraceResult))
  (bind _traceresult_2 (LocalVariables|GetTraceResult))
  (bind _returnvalue_5 (>= _angle 360))
  (bind _returnvalue_6 (/ 9e+02 _distance))
  (bind _returnvalue_7 (Math|Conversions|ToFloat(Integer) _angle_2))
  (bind _rootcomponent (Variables|/Script/Engine.Actor|GetRootComponent _returnvalue_2))
  (bind _rootcomponent_2 (Variables|/Script/Engine.Actor|GetRootComponent _returnvalue_3))
  (bind _rootcomponent_3 (Variables|/Script/Engine.Actor|GetRootComponent _returnvalue))
  (bind _returnvalue_8 (/ _returnvalue_7 -2.0))
  (bind _returnvalue_9 (Transformation|GetWorldLocation _rootcomponent_3))
  (bind _returnvalue_10 (Transformation|GetWorldLocation _rootcomponent_2))
  (bind _returnvalue_11 (Math|Vector|GetForwardVector _rootcomponent))
  (bind _returnvalue_12 (Math|Rotator|MakeRotator 0.0 0.0 _returnvalue_8))
  (bind _returnvalue_13 (Math|Vector|SelectVector "0,1.000000, 0" _returnvalue_11 _returnvalue_5))
  (bind _returnvalue_14 (+ _returnvalue_8 _pitch))
  (bind _returnvalue_15 (Math|Rotator|MakeRotator _returnvalue_14 0.0 0.0))
  (bind _returnvalue_16 (Utilities|Select :Index _lostype_2 :NewEnumerator0 _returnvalue_12 :NewEnumerator1 _returnvalue_15))
  (bind _returnvalue_17 (Math|Vector|RotateVector _returnvalue_13 _returnvalue_16))
  (Utilities|FlowControl|Sequence
    (:then_0
      ;[1 1 1] LineTrace
      (for _index (range 0 (Math|Float|Truncate (/ (Math|Conversions|ToFloat(Integer) (Variables|Default|GetAngle)) (Variables|Default|GetDegresPerTrace))))
        (bind (_outhit _returnvalue_18) (Collision|LineTraceByChannel _returnvalue_10 (+ (* (Utilities|Select :Index (Variables|Default|GetLosType) :NewEnumerator0 (Math|Vector|RotateVector _returnvalue_17 (Math|Rotator|MakeRotator 0.0 0.0 (* _index (Variables|Default|GetDegresPerTrace)))) :NewEnumerator1 (Math|Vector|RotateVector _returnvalue_17 (Math|Rotator|MakeRotator (* _index (Variables|Default|GetDegresPerTrace)) 0.0 0.0))) (Variables|Default|GetDistance)) _returnvalue_10) "TraceTypeQuery1" false (Variables|IgnoreMe|GetLOSActors) "None"))
        (if _returnvalue_18
          (if (Actor|ActorHasTag (.HitActor (Collision|BreakHitResult _outhit)) "LOS")
            (Utilities|Array|AddUnique (Variables|IgnoreMe|GetLOSActors) (.HitActor (Collision|BreakHitResult _outhit)))
            (LocalVariables|SetExtraDistance 1e+01 :!label _label)
            (Utilities|Array|Add _traceresult (+ (* (Utilities|Select :Index (Variables|Default|GetLosType) :NewEnumerator0 (Math|Vector|RotateVector _returnvalue_17 (Math|Rotator|MakeRotator 0.0 0.0 (* _index (Variables|Default|GetDegresPerTrace)))) :NewEnumerator1 (Math|Vector|RotateVector _returnvalue_17 (Math|Rotator|MakeRotator (* _index (Variables|Default|GetDegresPerTrace)) 0.0 0.0))) (LocalVariables|GetExtraDistance)) (+ (* (Utilities|Select :Index (Variables|Default|GetLosType) :NewEnumerator0 (Math|Vector|RotateVector _returnvalue_17 (Math|Rotator|MakeRotator 0.0 0.0 (* _index (Variables|Default|GetDegresPerTrace)))) :NewEnumerator1 (Math|Vector|RotateVector _returnvalue_17 (Math|Rotator|MakeRotator (* _index (Variables|Default|GetDegresPerTrace)) 0.0 0.0))) (Variables|Default|GetDistance)) _returnvalue_10)))
            (else
              (if (Actor|ActorHasTag (.HitActor (Collision|BreakHitResult _outhit)) "Loshit")
                (LocalVariables|SetExtraDistance (Math|Conversions|ToFloat(Integer) (Utilities|String|ToString(Name) (Utilities|Array|Get(acopy) (Variables|/Script/Engine.Actor|GetTags (.HitActor (Collision|BreakHitResult _outhit))) (+ (Utilities|Array|FindItem (Variables|/Script/Engine.Actor|GetTags (.HitActor (Collision|BreakHitResult _outhit))) "Loshit") 1)))))
                (else
                  (LocalVariables|SetExtraDistance 0.0)))
              (Utilities|Array|Add _traceresult (+ (* (Utilities|Select :Index (Variables|Default|GetLosType) :NewEnumerator0 (Math|Vector|RotateVector _returnvalue_17 (Math|Rotator|MakeRotator 0.0 0.0 (* _index (Variables|Default|GetDegresPerTrace)))) :NewEnumerator1 (Math|Vector|RotateVector _returnvalue_17 (Math|Rotator|MakeRotator (* _index (Variables|Default|GetDegresPerTrace)) 0.0 0.0))) (LocalVariables|GetExtraDistance)) (.Location (Collision|BreakHitResult _outhit))))))
          (else
            (goto _label)))))
    (:then_1
      ;[1 1 1] PreperaTiangles
      (for _index_2 (range 0 (- (Utilities|Array|Length (LocalVariables|GetTraceResult)) 2))
        (Utilities|Array|Add (LocalVariables|GetCanvansTri) (Utilities|Struct|MakeCanvasUVTri (Math|Conversions|ToVector2D(Vector) _returnvalue_4) "(X=0.000000,Y=0.000000)" "(R=1.000000,G=1.000000,B=1.000000,A=0.000000)" (Utilities|Select :Index _lostype :NewEnumerator0 (Math|Conversions|ToVector2D(Vector) (+ (* (- (Utilities|Array|Get(acopy) _traceresult_2 _index_2) _returnvalue_9) _returnvalue_6) _returnvalue_4)) :NewEnumerator1 (Math|Vector2D|MakeVector2D (.Y (Math|Vector|BreakVector (+ (* (- (Utilities|Array|Get(acopy) _traceresult_2 _index_2) _returnvalue_9) _returnvalue_6) _returnvalue_4))) (- 1.8e+03 (.Z (Math|Vector|BreakVector (+ (* (- (Utilities|Array|Get(acopy) _traceresult_2 _index_2) _returnvalue_9) _returnvalue_6) _returnvalue_4)))))) "(X=0.000000,Y=0.000000)" "(R=1.000000,G=1.000000,B=1.000000,A=0.000000)" (Utilities|Select :Index _lostype :NewEnumerator0 (Math|Conversions|ToVector2D(Vector) (+ (* (- (Utilities|Array|Get(acopy) _traceresult_2 (+ _index_2 1)) _returnvalue_9) _returnvalue_6) _returnvalue_4)) :NewEnumerator1 (Math|Vector2D|MakeVector2D (.Y (Math|Vector|BreakVector (+ (* (- (Utilities|Array|Get(acopy) _traceresult_2 (+ _index_2 1)) _returnvalue_9) _returnvalue_6) _returnvalue_4))) (- 1.8e+03 (.Z (Math|Vector|BreakVector (+ (* (- (Utilities|Array|Get(acopy) _traceresult_2 (+ _index_2 1)) _returnvalue_9) _returnvalue_6) _returnvalue_4)))))) "(X=0.000000,Y=0.000000)" "(R=1.000000,G=1.000000,B=1.000000,A=0.000000)"))))
    (:then_2
      ;[1 1 1] Draw
      (Rendering|ClearRenderTarget2D _losrendertarget)
      (bind (_canvas _size _context) (Rendering|BeginDrawCanvastoRenderTarget _losrendertarget))
      (Class|Canvas|DrawTriangle _canvas 0 (LocalVariables|GetCanvansTri))
      (Rendering|EndDrawCanvastoRenderTarget _context))))

(fn SetNewMaterial
  (params (Component :type Mesh%20Component%20Object%20Reference))
  (for (_array_element _array_index) (Rendering|Material|GetMaterials Component)
    (bind _asmaterial_instance_dynamic (Utilities|Casting|CastToMaterialInstanceDynamic _array_element)
      (:then
        (LocalVariables|SetDMI _asmaterial_instance_dynamic))
      (:CastFailed
        (bind _returnvalue (Rendering|Material|CreateDynamicMaterialInstance _array_element "None" :!class /Script/Engine.KismetMaterialLibrary))
        (LocalVariables|SetDMI _returnvalue)))
    (Rendering|Material|SetScalarParameterValue (LocalVariables|GetDMI) "Distance" (Variables|Default|GetDistance) :!class /Script/Engine.MaterialInstanceDynamic)
    (Rendering|Material|SetTextureParameterValue (LocalVariables|GetDMI) "Texture" (Utilities|Select :Index (Variables|IgnoreMe|GetPlayerID) :Option%200 "/Game/LineOfSightMP/Textures/RTC_LOS0.RTC_LOS0" :Option%201 "/Game/LineOfSightMP/Textures/RTC_LOS1.RTC_LOS1" :Option%202 "/Game/LineOfSightMP/Textures/RTC_LOS2.RTC_LOS2" :Option%203 "/Game/LineOfSightMP/Textures/RTC_LOS3.RTC_LOS3" :Option%204 "/Game/LineOfSightMP/Textures/RTC_LOS4.RTC_LOS4" :Option%205 "/Game/LineOfSightMP/Textures/RTC_LOS5.RTC_LOS5" :Option%206 "/Game/LineOfSightMP/Textures/RTC_LOS6.RTC_LOS6" :Option%207 "/Game/LineOfSightMP/Textures/RTC_LOS7.RTC_LOS7"))
    (Rendering|Material|SetScalarParameterValue (LocalVariables|GetDMI) "LOSEnable" 1.0 :!class /Script/Engine.MaterialInstanceDynamic)
    (Rendering|Material|SetMaterial Component _array_index (LocalVariables|GetDMI))))

(fn DisableforPlayer
  (params (Pawn :type Pawn%20Object%20Reference))
  (for _array_element (Actor|GetComponentsByClass Pawn "/Script/Engine.SkeletalMeshComponent")
    (LocalVariables|SetComponent _array_element)
    (for (_array_element_2 _array_index) (Rendering|Material|GetMaterials (LocalVariables|GetComponent))
      (bind _asmaterial_instance_dynamic (Utilities|Casting|CastToMaterialInstanceDynamic _array_element_2)
        (:then
          (LocalVariables|SetDMI _asmaterial_instance_dynamic))
        (:CastFailed
          (bind _returnvalue (Rendering|Material|CreateDynamicMaterialInstance _array_element_2 "None" :!class /Script/Engine.KismetMaterialLibrary))
          (LocalVariables|SetDMI _returnvalue)))
      (Rendering|Material|SetScalarParameterValue (LocalVariables|GetDMI) "LOSEnable" 0.0 :!class /Script/Engine.MaterialInstanceDynamic) ; Disable LOS
      (Rendering|Material|SetMaterial (LocalVariables|GetComponent) _array_index (LocalVariables|GetDMI))))
  (for _array_element_3 (Actor|GetComponentsByClass Pawn "/Script/Engine.StaticMeshComponent")
    (LocalVariables|SetComponent _array_element_3)
    (for (_array_element_4 _array_index_2) (Rendering|Material|GetMaterials (LocalVariables|GetComponent))
      (bind _asmaterial_instance_dynamic_2 (Utilities|Casting|CastToMaterialInstanceDynamic _array_element_4)
        (:then
          (LocalVariables|SetDMI _asmaterial_instance_dynamic_2))
        (:CastFailed
          (bind _returnvalue_2 (Rendering|Material|CreateDynamicMaterialInstance _array_element_4 "None" :!class /Script/Engine.KismetMaterialLibrary))
          (LocalVariables|SetDMI _returnvalue_2)))
      (Rendering|Material|SetScalarParameterValue (LocalVariables|GetDMI) "LOSEnable" 0.0 :!class /Script/Engine.MaterialInstanceDynamic) ; Disable LOS
      (Rendering|Material|SetMaterial (LocalVariables|GetComponent) _array_index_2 (LocalVariables|GetDMI)))))

(fn SetNewMaterialforEmmier
  (params (InputPin :type Primitive%20Component%20Object%20Reference))
  (for _index (range 0 (- (Rendering|Material|GetNumMaterials InputPin) 1))
    (bind _asmaterial_instance_dynamic (Utilities|Casting|CastToMaterialInstanceDynamic (Rendering|Material|GetMaterial InputPin _index))
      (:then
        (LocalVariables|SetDMI _asmaterial_instance_dynamic))
      (:CastFailed
        (bind _returnvalue (Rendering|Material|CreateDynamicMaterialInstance (Rendering|Material|GetMaterial InputPin _index) "None" :!class /Script/Engine.KismetMaterialLibrary))
        (LocalVariables|SetDMI _returnvalue)))
    (Rendering|Material|SetScalarParameterValue (LocalVariables|GetDMI) "Distance" (Variables|Default|GetDistance) :!class /Script/Engine.MaterialInstanceDynamic)
    (Rendering|Material|SetTextureParameterValue (LocalVariables|GetDMI) "Texture" (Utilities|Select :Index (Variables|IgnoreMe|GetPlayerID) :Option%200 "/Game/LineOfSightMP/Textures/RTC_LOS0.RTC_LOS0" :Option%201 "/Game/LineOfSightMP/Textures/RTC_LOS1.RTC_LOS1" :Option%202 "/Game/LineOfSightMP/Textures/RTC_LOS2.RTC_LOS2" :Option%203 "/Game/LineOfSightMP/Textures/RTC_LOS3.RTC_LOS3" :Option%204 "/Game/LineOfSightMP/Textures/RTC_LOS4.RTC_LOS4" :Option%205 "/Game/LineOfSightMP/Textures/RTC_LOS5.RTC_LOS5" :Option%206 "/Game/LineOfSightMP/Textures/RTC_LOS6.RTC_LOS6" :Option%207 "/Game/LineOfSightMP/Textures/RTC_LOS7.RTC_LOS7"))
    (Rendering|Material|SetScalarParameterValue (LocalVariables|GetDMI) "LOSEnable" 1.0 :!class /Script/Engine.MaterialInstanceDynamic)
    (Rendering|Material|SetMaterial InputPin _index (LocalVariables|GetDMI))))