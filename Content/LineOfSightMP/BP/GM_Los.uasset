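; GM_Los is a game mode that tracks connected player controllers for a multiplayer line-of-sight system.
; PostLogin adds each controller to Players and runs the update loop after a short retriggerable delay, and logout removes the controller without refreshing.
; The loop, also exposed as an Update event, passes each player's array index to the AC_Los component on its controlled pawn.
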(event Custom|Update
  (for (_array_element _array_index) (Variables|Default|GetPlayers)
    (Utilities|IsValid (Pawn|GetControlledPawn _array_element)
      (:Is%20Valid
        (Utilities|IsValid (Actor|GetComponentbyClass (Pawn|GetControlledPawn _array_element) "/Game/LineOfSightMP/BP/AC_Los.AC_Los_C")
          (:Is%20Valid
            (Default|Update (Actor|GetComponentbyClass (Pawn|GetControlledPawn _array_element) "/Game/LineOfSightMP/BP/AC_Los.AC_Los_C") _array_index)))))))

(event EventPostLogin
  (params (NewPlayer :type Player%20Controller%20Object%20Reference))
  (bind _players (Variables|Default|GetPlayers))
  (Utilities|Array|Add _players NewPlayer)
  (Utilities|FlowControl|RetriggerableDelay 0.5)
  (for (_array_element _array_index) _players
    (Utilities|IsValid (Pawn|GetControlledPawn _array_element)
      (:Is%20Valid
        (Utilities|IsValid (Actor|GetComponentbyClass (Pawn|GetControlledPawn _array_element) "/Game/LineOfSightMP/BP/AC_Los.AC_Los_C")
          (:Is%20Valid
            (Default|Update (Actor|GetComponentbyClass (Pawn|GetControlledPawn _array_element) "/Game/LineOfSightMP/BP/AC_Los.AC_Los_C") _array_index)))))))

(event EventOnLogout
  (params (ExitingController :type Controller%20Object%20Reference))
  (bind _asplayer_controller (Utilities|Casting|CastToPlayerController ExitingController))
  (Utilities|Array|RemoveItem (Variables|Default|GetPlayers) _asplayer_controller))

(fn ConstructionScript)